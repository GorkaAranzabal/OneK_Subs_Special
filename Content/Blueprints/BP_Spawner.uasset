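; BP_Spawner is an enemy spawner that sends out waves of BP_Enemy from its own transform.
; BeginPlay spawns a wave immediately, then loops on a retriggerable delay to start another wave every few seconds.
; Each wave is a custom event that spawns three enemies in sequence, staggered by short delays.
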(event `self.ReceiveBeginPlay`
  ;[0 0.4342 1] Spawner Logic
  (`self.Spawn Wave Enemy`)
  (`KismetSystemLibrary.RetriggerableDelay` 5.0 :!label _label)
  (`self.Spawn Wave Enemy`)
  (goto _label))

(event `Spawn Wave Enemy`
  ;[0 0.4342 1] Spawner Logic
  (`|SpawnActorFromClass` "/Game/Blueprints/BP_Enemy.BP_Enemy_C" (`self.GetTransform`) "Undefined" "OverrideRootScale" null null)
  (`KismetSystemLibrary.Delay` 0.7)
  (`|SpawnActorFromClass` "/Game/Blueprints/BP_Enemy.BP_Enemy_C" (`self.GetTransform`) "Undefined" "OverrideRootScale" null null)
  (`KismetSystemLibrary.Delay` 0.7)
  (`|SpawnActorFromClass` "/Game/Blueprints/BP_Enemy.BP_Enemy_C" (`self.GetTransform`) "Undefined" "OverrideRootScale" null null))

(fn `UserConstructionScript`)